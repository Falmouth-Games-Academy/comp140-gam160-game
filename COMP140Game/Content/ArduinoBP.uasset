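; ArduinoBP is an actor that parses an input string, apparently Arduino data, into a set of string values.
; Shortly after BeginPlay it stores the first InputController actor, though its graphs never use that reference.
; Each tick it splits InputString on "s", prints the segment count, and stores the first segment with exactly five comma-separated fields in StringValues.
; Nothing in these graphs fills InputString or reads StringValues.
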(event EventBeginPlay
  (Utilities|FlowControl|Delay 0.2)
  (bind _outactors (Actor|GetAllActorsOfClass "/Game/InputController.InputController_C"))
  (Variables|Default|SetInputController (Utilities|Array|Get(acopy) _outactors)))

(event Collision|EventActorBeginOverlap
  (params (OtherActor :type Actor%20Object%20Reference)))

(event EventTick
  (params (DeltaSeconds :type Float%20%28single-precision%29))
  (bind _inputstring (Variables|Default|GetInputString))
  (bind _returnvalue (Utilities|String|ParseIntoArray _inputstring "s"))
  (Development|PrintString (Utilities|String|ToString(Integer) (Utilities|Array|Length _returnvalue)))
  (bind _array_element (Utilities|Array|ForEachLoopwithBreak _returnvalue :!label _label)
    (:LoopBody
      (if (== (Utilities|Array|Length (Utilities|String|ParseIntoArray _array_element ",")) 5)
        (Variables|Default|SetStringValues (Utilities|String|ParseIntoArray _array_element ","))
        (goto _label Break)))))

(fn ConstructionScript)